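; BP_BaseDestroyableObject is a base actor for objects that can be destroyed when their health runs out.
; On BeginPlay it binds a handler to the health-changed event of its BPHealthComponent.
; The handler writes the health percentage to the progress bar of the HealthBar in its Widget, then destroys the actor if the component reports death.
; The death check runs only if the widget cast to HealthBar succeeds.
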(event `self.ReceiveBeginPlay`
  (add `/Game/BluePrints/BP_HealthComponent.OnHealthChanged` (`self.BP_HealthComponent`) (delegate `OnHealthChanged_Event`)))

(event `OnHealthChanged_Event`
  (bind _bp_healthcomponent (`self.BP_HealthComponent`))
  (bind _ashealth_bar (cast `/Game/UI/HealthBar` (`WidgetComponent.GetWidget` (`self.Widget`))))
  (`ProgressBar.SetPercent` (`/Game/UI/HealthBar.HealthProgressBar` _ashealth_bar) (`/Game/BluePrints/BP_HealthComponent.HealthPercentage` _bp_healthcomponent))
  (if (`/Game/BluePrints/BP_HealthComponent.Died` _bp_healthcomponent)
    (`self.K2_DestroyActor`)))

(fn `UserConstructionScript`)